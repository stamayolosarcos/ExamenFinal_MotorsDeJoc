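; CoinDoor_BP is a door that opens for a ThirdPersonCharacter holding at least CoinsNeeded coins, without deducting them.
; On actor overlap it checks the coin count, or an Open flag that bypasses the check and is then cleared.
; It instantly shifts the StaticMesh 200 units along world X and disables Box collision.
; After a two-second delay it moves the mesh back and restores collision.
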(event EventBeginPlay)

(event Collision|EventActorBeginOverlap
  (params (OtherActor :type Actor%20Object%20Reference))
  (bind _staticmesh (Variables|Default|GetStaticMesh))
  (bind _staticmesh_2 (Variables|Default|GetStaticMesh))
  (bind _returnvalue (Transformation|GetWorldLocation _staticmesh))
  (bind _returnvalue_2 (Transformation|GetWorldLocation _staticmesh_2))
  (bind _asthird_person_character (Utilities|Casting|CastToThirdPersonCharacter OtherActor))
  (if (or (>= (Variables|/Game/ThirdPersonBP/Blueprints/ThirdPersonCharacter.ThirdPersonCharacter_C|GetCoins _asthird_person_character) (Variables|Default|GetCoinsNeeded)) (Variables|Default|GetOpen))
    (Variables|Default|SetOpen false)
    (Transformation|SetWorldLocation _staticmesh_2 (Math|Vector|MakeVector (+ (.x _returnvalue_2) 2e+02) (.y _returnvalue_2) (.z _returnvalue_2)) false false)
    (Collision|SetCollisionEnabled (Variables|Default|GetBox) "NoCollision")
    (Utilities|FlowControl|Delay 2.0)
    (Transformation|SetWorldLocation _staticmesh (Math|Vector|MakeVector (- (.x _returnvalue) 2e+02) (.y _returnvalue) (.z _returnvalue)) false false)
    (Collision|SetCollisionEnabled (Variables|Default|GetBox) "QueryAndPhysics")))

(event EventTick
  (params (DeltaSeconds :type Float%20%28single-precision%29)))

(fn ConstructionScript)